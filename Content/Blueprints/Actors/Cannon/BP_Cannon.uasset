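; Cannon actor that automatically fires projectiles on a repeating cycle from BeginPlay.
; After a fire-rate delay it spawns a scaled BP_Projectile at the ProjectileSpawnPoint transform, then plays a timeline from the start.
; The timeline drives the turret mesh's relative Y location to animate the barrel, and its Cannon Fired event track loops back to the delay for the next shot.
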(event EventBeginPlay
  (Utilities|FlowControl|Delay (Variables|CannonProperties|GetCanonFireRate) :!label _label)
  (CallFunction|SpawnProjectile)
  (bind _cannon_turret_location (Timeline|TimelineCannonFiring PlayFromStart)
    (:Update
      (CallFunction|MoveCannonBarrel _cannon_turret_location))
    (:Cannon%20Fired
      (goto _label))))

(fn ConstructionScript)

(fn SpawnProjectile
  (bind _projectilespawnpoint (Variables|Default|GetProjectileSpawnPoint))
  (Game|SpawnActorfromClass "/Game/Blueprints/Actors/Projectiles/BP_Projectile.BP_Projectile_C" (Math|Transform|MakeTransform (Transformation|GetWorldLocation _projectilespawnpoint) (Transformation|GetWorldRotation _projectilespawnpoint) (Math|Conversions|ToVector(Float) (Variables|CannonProperties|GetProjectileScale))) "Undefined" 0 0))

(fn MoveCannonBarrel
  (params (CannonBarrel%20Y%20Location :type Float%20%28single-precision%29))
  (Transformation|SetRelativeLocation (Variables|Default|GetMeshCannonTurret) (Math|Vector|MakeVector 0.0 CannonBarrel%20Y%20Location 0.0) false false))